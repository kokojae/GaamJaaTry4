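; Player controller for an RTS camera that handles panning and zooming of the camera pawn.
; On BeginPlay it casts and caches the player pawn as the RTS camera pawn.
; Move axes feed its floating movement component along world X and Y, independent of camera rotation.
; Zoom inputs step the spring arm length within clamped limits, and a reset input restores a fixed default length.
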(event `self.ReceiveBeginPlay`
  (`self.ReferenceCast`))

(event `InputAction|ZoomIn`
  (params (Key :type "Key Structure"))
  (bind _springarm (`/Game/RTS_Tutorial/BluePrints/BP_RTS_CameraPawn.SpringArm` (`self.CameraPawnRef`)))
  ;[1 1 1] Zoom Controls
  ;;[1 1 1] Zoom In
  (:`Pressed`
    (set `SpringArmComponent.TargetArmLength` (`KismetMathLibrary.FClamp` (- (`SpringArmComponent.TargetArmLength` _springarm) (`self.ZoomSpeed`)) (`self.MinZoomLimit`) (`self.MaxZoomLimit`)) _springarm)))

(event `InputAxis|MoveForward`
  (params (AxisValue :type "Float (single-precision)"))
  (`PawnMovementComponent.AddInputVector` (`/Game/RTS_Tutorial/BluePrints/BP_RTS_CameraPawn.FloatingPawnMovement` (`self.CameraPawnRef`)) (`KismetMathLibrary.MakeVector` AxisValue) false))

(event `InputAction|ZoomReset`
  (params (Key :type "Key Structure"))
  ;[1 1 1] Zoom Controls
  ;;[1 1 1] Zoom Reset
  (:`Pressed`
    (set `SpringArmComponent.TargetArmLength` 1500.0 (`/Game/RTS_Tutorial/BluePrints/BP_RTS_CameraPawn.SpringArm` (`self.CameraPawnRef`)))))

(event `InputAxis|MoveRight`
  (params (AxisValue :type "Float (single-precision)"))
  (`PawnMovementComponent.AddInputVector` (`/Game/RTS_Tutorial/BluePrints/BP_RTS_CameraPawn.FloatingPawnMovement` (`self.CameraPawnRef`)) (`KismetMathLibrary.MakeVector` 0.0 AxisValue) false))

(event `InputAction|ZoomOut`
  (params (Key :type "Key Structure"))
  (bind _springarm (`/Game/RTS_Tutorial/BluePrints/BP_RTS_CameraPawn.SpringArm` (`self.CameraPawnRef`)))
  ;[1 1 1] Zoom Controls
  ;;[1 1 1] Zoom Out
  (:`Pressed`
    (set `SpringArmComponent.TargetArmLength` (`KismetMathLibrary.FClamp` (+ (`self.ZoomSpeed`) (`SpringArmComponent.TargetArmLength` _springarm)) (`self.MinZoomLimit`) (`self.MaxZoomLimit`)) _springarm)))

(fn `UserConstructionScript`)